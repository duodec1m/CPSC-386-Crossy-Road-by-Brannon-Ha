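; Spawning_Floor is a floor segment actor that can chain to the next segment and removes itself after the chicken player passes.
; When a Chicken_Move actor overlaps EndTrigger, it waits two seconds, decrements the Straights counter on My_GameMode, and destroys itself.
; GetAttach returns the world transform of the Attach component, exposing a connection point for placing another piece.
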(event OnComponentBeginOverlap(EndTrigger)
  (params (OverlappedComponent :type Primitive%20Component%20Object%20Reference) (OtherActor :type Actor%20Object%20Reference) (OtherComp :type Primitive%20Component%20Object%20Reference) (OtherBodyIndex :type Integer) (bFromSweep :type Boolean) (SweepResult :type Hit%20Result%20Structure%20%28by%20ref%29))
  (Utilities|Casting|CastToChicken_Move OtherActor)
  (Utilities|FlowControl|Delay 2.0)
  (bind _asmy_game_mode (Utilities|Casting|CastToMy_GameMode (Game|GetGameMode)))
  (Variables|/Game/Blueprints/My_GameMode.My_GameMode_C|SetStraights _asmy_game_mode (- (Variables|/Game/Blueprints/My_GameMode.My_GameMode_C|GetStraights _asmy_game_mode) 1))
  (Actor|DestroyActor))

(fn ConstructionScript)

(fn GetAttach
  (return (Transformation|GetWorldTransform (Variables|Default|GetAttach))))