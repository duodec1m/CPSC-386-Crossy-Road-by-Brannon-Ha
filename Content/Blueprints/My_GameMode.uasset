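; Game mode that procedurally builds a Crossy Road-style level of chained floor pieces and hazard rows.
; Tick tops up floors and rows to fixed counts, chaining each floor from the previous one's attach point.
; SpawnVehicle randomly picks side and row type (car, truck, train, river, trees/rocks), then advances along X.
; Cars, trucks and logs spawn as same-speed pairs, rivers may get lilypads instead, and trains reference their railroad.
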(event EventBeginPlay)

(event EventTick
  (params (DeltaSeconds :type Float%20%28single-precision%29))
  (if (< (Variables|Default|GetStraights) 5)
    (CallFunction|AddFloor))
  (if (< (Variables|Default|GetVehicle%20Rows) 30)
    (CallFunction|SpawnVehicle)))

(fn ConstructionScript)

(fn AddFloor
  (bind _returnvalue (Game|SpawnActorfromClass "/Game/Blueprints/Spawning_Floor.Spawning_Floor_C" (Variables|Default|GetNextSpawn) "Undefined" 0 0))
  (bind _attach (Default|GetAttach _returnvalue))
  (Variables|Default|SetNextSpawn _attach)
  (Variables|Default|SetStraights (+ (Variables|Default|GetStraights) 1)))

(fn SpawnVehicle
  (if (> (Math|Random|RandomIntegerinRange 0 100) 50)
    (Variables|Default|SetY_Spawn -496.0)
    (Variables|Default|SetLookDirection 0.0)
    (else
      (Variables|Default|SetY_Spawn 496.0)
      (Variables|Default|SetLookDirection 1.8e+02)))
  (switch int (Math|Random|RandomIntegerinRange 0 4)
    (:Default
      (bind _location_x (CallFunction|SpawnCarRow (Math|Transform|MakeTransform (Math|Vector|MakeVector (Variables|Default|GetLast%20Spawned%20Vehicle%20X) (Variables|Default|GetY_Spawn) 48.0) (Math|Rotator|MakeRotator 0.0 0.0 (Variables|Default|GetLookDirection))) :!label _label))
      (Game|SpawnActorfromClass "/Game/Blueprints/Road.Road_C" (Math|Transform|MakeTransform (Math|Vector|MakeVector _location_x -496.0 15.0) "0.000000,90.000000, 0" "12.000000,5.000000,5.000000") "Undefined" 0 0)
      (Variables|Default|SetLast%20Spawned%20Vehicle%20X (+ (Variables|Default|GetLast%20Spawned%20Vehicle%20X) 1e+02)))
    (:0
      (bind (_train _location_x_2) (CallFunction|SpawnTrainRow (Math|Transform|MakeTransform (Math|Vector|MakeVector (Variables|Default|GetLast%20Spawned%20Vehicle%20X) (Variables|Default|GetY_Spawn) 48.0) (Math|Rotator|MakeRotator 0.0 0.0 (Variables|Default|GetLookDirection)))))
      (bind _returnvalue (Game|SpawnActorfromClass "/Game/Blueprints/RailRoad.RailRoad_C" (Math|Transform|MakeTransform (Math|Vector|MakeVector _location_x_2 -496.0 15.0) "0.000000,90.000000, 0" "12.000000,5.000000,5.000000") "Undefined" 0 0))
      (Variables|/Game/Blueprints/Train_Move.Train_Move_C|SetRailroad%20Child _train _returnvalue)
      (Variables|Default|SetLast%20Spawned%20Vehicle%20X (+ (Variables|Default|GetLast%20Spawned%20Vehicle%20X) 1e+02)))
    (:1
      (bind _location_x_3 (CallFunction|SpawnTruckRow (Math|Transform|MakeTransform (Math|Vector|MakeVector (Variables|Default|GetLast%20Spawned%20Vehicle%20X) (Variables|Default|GetY_Spawn) 48.0) (Math|Rotator|MakeRotator 0.0 0.0 (Variables|Default|GetLookDirection)))))
      (Game|SpawnActorfromClass "/Game/Blueprints/Road.Road_C" (Math|Transform|MakeTransform (Math|Vector|MakeVector _location_x_3 -496.0 15.0) "0.000000,90.000000, 0" "12.000000,5.000000,5.000000") "Undefined" 0 0)
      (Variables|Default|SetLast%20Spawned%20Vehicle%20X (+ (Variables|Default|GetLast%20Spawned%20Vehicle%20X) 1e+02)))
    (:2
      (goto _label))
    (:3
      (bind _location_x_4 (CallFunction|SpawnRiver (Math|Transform|MakeTransform (Math|Vector|MakeVector (Variables|Default|GetLast%20Spawned%20Vehicle%20X) (Variables|Default|GetY_Spawn) 48.0) (Math|Rotator|MakeRotator 0.0 0.0 (Variables|Default|GetLookDirection)))))
      (Game|SpawnActorfromClass "/Game/Blueprints/Water.Water_C" (Math|Transform|MakeTransform (Math|Vector|MakeVector _location_x_4 -496.0 15.0) "0.000000,90.000000, 0" "12.000000,5.000000,5.000000") "Undefined" 0 0)
      (Variables|Default|SetLast%20Spawned%20Vehicle%20X (+ (Variables|Default|GetLast%20Spawned%20Vehicle%20X) 1e+02)))
    (:4
      (CallFunction|SpawnTreeRow (Math|Transform|MakeTransform (Math|Vector|MakeVector (Variables|Default|GetLast%20Spawned%20Vehicle%20X) (Variables|Default|GetY_Spawn) 48.0) (Math|Rotator|MakeRotator 0.0 0.0 (Variables|Default|GetLookDirection))))
      (Variables|Default|SetLast%20Spawned%20Vehicle%20X (+ (Variables|Default|GetLast%20Spawned%20Vehicle%20X) 1e+02))))
  (Variables|Default|SetVehicle%20Rows (+ (Variables|Default|GetVehicle%20Rows) 1)))

(fn SpawnTrainRow
  (params (Location :type Transform))
  (bind _returnvalue (Game|SpawnActorfromClass "/Game/Blueprints/Train_Move.Train_Move_C" (Math|Transform|MakeTransform (Math|Vector|MakeVector (.x (.location Location)) (.y (.location Location)) 38.0) (.rotation Location) (.scale Location)) "AlwaysSpawn" 0 0))
  (return _returnvalue (.x (.location Location))))

(fn SpawnCarRow
  (params (Location :type Transform))
  (bind _returnvalue (Game|SpawnActorfromClass "/Game/Blueprints/Car_Move.Car_Move_C" (Math|Transform|MakeTransform (Math|Vector|MakeVector (.x (.location Location)) (.y (.location Location)) 42.150002) (.rotation Location) (.scale Location)) "AlwaysSpawn" 0 0))
  (bind _output_get (Variables|/Game/Blueprints/Car_Move.Car_Move_C|SetSpeed _returnvalue (Math|Random|RandomFloatinRange 1e+02 3e+02)))
  (bind _returnvalue_2 (Game|SpawnActorfromClass "/Game/Blueprints/Car_Move.Car_Move_C" (Math|Transform|MakeTransform (Math|Vector|MakeVector (.x (.location Location)) 0.0 42.150002) (.rotation Location) (.scale Location)) "AlwaysSpawn" 0 0))
  (Variables|/Game/Blueprints/Car_Move.Car_Move_C|SetSpeed _returnvalue_2 _output_get)
  (return (.x (.location Location))))

(fn SpawnTruckRow
  (params (Location :type Transform))
  (bind _returnvalue (Game|SpawnActorfromClass "/Game/Blueprints/Truck_Move.Truck_Move_C" (Math|Transform|MakeTransform (Math|Vector|MakeVector (.x (.location Location)) (.y (.location Location)) 58.650002) (.rotation Location) (.scale Location)) "AlwaysSpawn" 0 0))
  (bind _output_get (Variables|/Game/Blueprints/Truck_Move.Truck_Move_C|SetSpeed _returnvalue (Math|Random|RandomFloatinRange 1e+02 3e+02)))
  (bind _returnvalue_2 (Game|SpawnActorfromClass "/Game/Blueprints/Truck_Move.Truck_Move_C" (Math|Transform|MakeTransform (Math|Vector|MakeVector (.x (.location Location)) 0.0 58.650002) (.rotation Location) (.scale Location)) "AlwaysSpawn" 0 0))
  (Variables|/Game/Blueprints/Truck_Move.Truck_Move_C|SetSpeed _returnvalue_2 _output_get)
  (return (.x (.location Location))))

(fn SpawnRiver
  (params (Location :type Transform))
  (if (> (Math|Random|RandomIntegerinRange 0 100) 50)
    (bind _returnvalue (Game|SpawnActorfromClass "/Game/Blueprints/Log_Move.Log_Move_C" (Math|Transform|MakeTransform (Math|Vector|MakeVector (.x (.location Location)) (.y (.location Location)) 0.0) (.rotation Location) (.scale Location)) "AlwaysSpawn" 0 0))
    (bind _output_get (Variables|/Game/Blueprints/Log_Move.Log_Move_C|SetSpeed _returnvalue (Math|Random|RandomFloatinRange 1e+02 3e+02)))
    (bind _returnvalue_2 (Game|SpawnActorfromClass "/Game/Blueprints/Log_Move.Log_Move_C" (Math|Transform|MakeTransform (Math|Vector|MakeVector (.x (.location Location)) 0.0 0.0) (.rotation Location) (.scale Location)) "AlwaysSpawn" 0 0))
    (Variables|/Game/Blueprints/Log_Move.Log_Move_C|SetSpeed _returnvalue_2 _output_get)
    (else
      (for _index (range -5 5)
        (if (< (Math|Random|RandomIntegerinRange 0 100) 30)
          (Game|SpawnActorfromClass "/Game/Blueprints/Lilypad.Lilypad_C" (Math|Transform|MakeTransform (Math|Vector|MakeVector (.x (.location Location)) (Math|Conversions|ToFloat(Integer) (* _index 100)) 16.0) (.rotation Location) (.scale Location)) "AlwaysSpawn" 0 0)))))
  (return (.x (.location Location))))

(fn SpawnTreeRow
  (params (Location :type Transform))
  (for _index (range -4 4)
    (if (< (Math|Random|RandomIntegerinRange 0 100) 30)
      (if (< (Math|Random|RandomIntegerinRange 0 100) 50)
        (Game|SpawnActorfromClass "/Game/Blueprints/Rock.Rock_C" (Math|Transform|MakeTransform (Math|Vector|MakeVector (.x (.location Location)) (Math|Conversions|ToFloat(Integer) (* _index 100)) 0.0) (.rotation Location) (.scale Location)) "AlwaysSpawn" 0 0)
        (else
          (Game|SpawnActorfromClass "/Game/Blueprints/Tree.Tree_C" (Math|Transform|MakeTransform (Math|Vector|MakeVector (.x (.location Location)) (Math|Conversions|ToFloat(Integer) (* _index 100)) 0.0) (.rotation Location) (.scale Location)) "AlwaysSpawn" 0 0)))))
  (Game|SpawnActorfromClass "/Game/Blueprints/Tree.Tree_C" (Math|Transform|MakeTransform (Math|Vector|MakeVector (.x (.location Location)) -5e+02 0.0) (.rotation Location) (.scale Location)) "AlwaysSpawn" 0 0)
  (Game|SpawnActorfromClass "/Game/Blueprints/Tree.Tree_C" (Math|Transform|MakeTransform (Math|Vector|MakeVector (.x (.location Location)) 5e+02 0.0) (.rotation Location) (.scale Location)) "AlwaysSpawn" 0 0))