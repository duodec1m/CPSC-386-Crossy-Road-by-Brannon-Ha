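; Eagle actor that swoops at the spot where the player character stood when it began play.
; On BeginPlay it sets a fixed rotation and captures that position once, so it does not home in on the player.
; Tick moves it there at constant speed with VInterpToConstant, then carries it onward along its local forward axis at the same speed, without sweep collision.
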(event EventBeginPlay
  (Variables|Default|SetLocation%20Placeholder (Transformation|GetActorLocation))
  (Transformation|SetActorRotation "0,180.000000, 0")
  (Variables|Default|SetDestination (Transformation|GetActorLocation (Game|GetPlayerCharacter 0))))

(event EventTick
  (params (DeltaSeconds :type Float%20%28single-precision%29))
  (bind _destination (Variables|Default|GetDestination))
  (if (Math|Vector|Equal(Vector) (- (Variables|Default|GetLocation%20Placeholder) _destination) "0, 0, 0" 5.0)
    (Transformation|AddActorLocalOffset (* "1750.000000,0.000000, 0" DeltaSeconds) false false)
    (else
      (bind _output_get (Variables|Default|SetLocation%20Placeholder (Math|Interpolation|VInterptoConstant (Variables|Default|GetLocation%20Placeholder) _destination DeltaSeconds 1.75e+03)))
      (Transformation|SetActorLocation _output_get false false))))

(fn ConstructionScript)