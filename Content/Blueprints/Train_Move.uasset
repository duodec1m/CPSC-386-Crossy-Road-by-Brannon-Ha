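; Train hazard that repeatedly runs along Y across a railroad row, with crossing warnings before each pass.
; Tick moves it along local Y; out of bounds, it waits randomly, triggers the RailroadChild sound and lights, then jumps to the opposite edge, playing its own audio and switching the lights off.
; Once the player is far enough ahead in X, it decrements My_GameMode's VehicleRows and destroys itself.
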(event EventTick
  (params (DeltaSeconds :type Float%20%28single-precision%29))
  (bind _returnvalue (Transformation|GetActorLocation))
  (bind _returnvalue_2 (Transformation|GetActorLocation))
  (bind _railroad_child (Variables|Default|GetRailroad%20Child))
  (bind _audio (Variables|/Game/Blueprints/RailRoad.RailRoad_C|GetAudio _railroad_child))
  (if (> (.x (Transformation|GetActorLocation (Game|GetPlayerCharacter 0))) (+ (.x (Transformation|GetActorLocation)) 1e+03))
    (CallFunction|DestroySelf)
    (else
      (Transformation|AddActorLocalOffset (* "0.000000,2000.000000, 0" DeltaSeconds) false false)
      (if (> (.y _returnvalue) 496.0)
        (Utilities|FlowControl|Delay (Math|Random|RandomFloatinRange 4.0 8.0))
        (Variables|Default|SetArriving true)
        (Audio|Components|Audio|Play _audio 0.0)
        (CallFunction|ToggleLights)
        (Utilities|FlowControl|Delay 1.5)
        (Transformation|SetActorLocation (Math|Vector|MakeVector (.x _returnvalue) -496.0 (.z _returnvalue)) false false)
        (Audio|Components|Audio|Play (Variables|Default|GetAudio) 0.0 :!label _label)
        (Variables|Default|SetArriving false)
        (CallFunction|ToggleLights)
        (elif (< (.y _returnvalue_2) -496.0)
          (Utilities|FlowControl|Delay (Math|Random|RandomFloatinRange 4.0 8.0))
          (Variables|Default|SetArriving true)
          (Audio|Components|Audio|Play _audio 0.0)
          (CallFunction|ToggleLights)
          (Utilities|FlowControl|Delay 1.5)
          (Transformation|SetActorLocation (Math|Vector|MakeVector (.x _returnvalue_2) 496.0 (.z _returnvalue_2)) false false)
          (goto _label))))))

(fn ConstructionScript)

(fn DestroySelf
  (bind _asmy_game_mode (Utilities|Casting|CastToMy_GameMode (Game|GetGameMode)))
  (Variables|/Game/Blueprints/My_GameMode.My_GameMode_C|SetVehicle%20Rows _asmy_game_mode (- (Variables|/Game/Blueprints/My_GameMode.My_GameMode_C|GetVehicle%20Rows _asmy_game_mode) 1))
  (Actor|DestroyActor))

(fn ToggleLights
  (bind _arriving (Variables|Default|GetArriving))
  (bind _railroad_child (Variables|Default|GetRailroad%20Child))
  (Rendering|SetVisibility (Variables|/Game/Blueprints/RailRoad.RailRoad_C|GetPointLight _railroad_child) _arriving false)
  (Rendering|SetVisibility (Variables|/Game/Blueprints/RailRoad.RailRoad_C|GetPointLight1 _railroad_child) _arriving false))