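; Truck_Move is a traffic vehicle that drives across a lane along its local Y axis at its Speed.
; Each Tick it moves without sweep, wraps to the opposite edge when world Y leaves the fixed bounds, and rarely plays a random car horn.
; Once the player is far enough ahead in X, it decrements VehicleRows on My_GameMode and destroys itself.
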(event EventTick
  (params (DeltaSeconds :type Float%20%28single-precision%29))
  (if (> (.x (Transformation|GetActorLocation (Game|GetPlayerCharacter 0))) (+ (.x (Transformation|GetActorLocation)) 1e+03))
    (CallFunction|DestroySelf)
    (else
      (Transformation|AddActorLocalOffset (* (Math|Vector|MakeVector 0.0 (Variables|Default|GetSpeed) 0.0) DeltaSeconds) false false)
      (CallFunction|ResetPosition)
      (if (< (Math|Random|RandomFloatinRange 0.0 1e+02) 0.01)
        (Audio|PlaySound2D "/Game/Sounds/car-horn.car-horn" 1.0 1.0 0.0 0 0)))))

(fn ConstructionScript)

(fn DestroySelf
  (bind _asmy_game_mode (Utilities|Casting|CastToMy_GameMode (Game|GetGameMode)))
  (Variables|/Game/Blueprints/My_GameMode.My_GameMode_C|SetVehicle%20Rows _asmy_game_mode (- (Variables|/Game/Blueprints/My_GameMode.My_GameMode_C|GetVehicle%20Rows _asmy_game_mode) 1))
  (Actor|DestroyActor))

(fn ResetPosition
  (bind _returnvalue (Transformation|GetActorLocation))
  (bind _returnvalue_2 (Transformation|GetActorLocation))
  (if (> (.y _returnvalue) 496.0)
    (Transformation|SetActorLocation (Math|Vector|MakeVector (.x _returnvalue) -496.0 (.z _returnvalue)) false false)
    (elif (< (.y _returnvalue_2) -496.0)
      (Transformation|SetActorLocation (Math|Vector|MakeVector (.x _returnvalue_2) 496.0 (.z _returnvalue_2)) false false))))