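; RailRoad is an actor, apparently a track segment, that removes itself once the player has moved past it along the X axis.
; BeginPlay hides its two point lights.
; Tick compares the player character's X position with its own and destroys the actor when the player is over 1000 units further along +X.
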(event EventBeginPlay
  (Rendering|SetVisibility (Variables|Default|GetPointLight1) false false)
  (Rendering|SetVisibility (Variables|Default|GetPointLight) false false))

(event EventTick
  (params (DeltaSeconds :type Float%20%28single-precision%29))
  (if (> (.x (Transformation|GetActorLocation (Game|GetPlayerCharacter 0))) (+ (.x (Transformation|GetActorLocation)) 1e+03))
    (Actor|DestroyActor)))

(fn ConstructionScript)