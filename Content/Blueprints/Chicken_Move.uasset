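; Player chicken for a Crossy Road-style game, hopping on a step grid with squash, cluck sounds and a score from furthest forward distance.
; Input sets target position and rotation that Tick interpolates toward, reverting blocked moves and letting logs carry the chicken sideways.
; A detached camera creeps forward, spawning a killer eagle when too close.
; Hit events handle vehicle, train and water deaths, plus log and lilypad landings.
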(event EventBeginPlay
  (Transformation|SetAbsolute (Variables|Default|GetCamera) true true false)
  (bind _output_get (Variables|Default|SetNew%20Position (Transformation|GetActorLocation)))
  (Variables|Default|SetLocation%20Placeholder _output_get)
  (Variables|Default|SetCamera%20Rotation%20Placeholder (Transformation|GetWorldRotation (Variables|Default|GetCamera)))
  (bind _returnvalue (Game|ConstructObjectfromClass "/Game/Blueprints/UIStuff/Score.Score_C" (Game|GetPlayerController 0)))
  (UserInterface|Viewport|AddtoViewport _returnvalue 0))

(event EventTick
  (params (DeltaSeconds :type Float%20%28single-precision%29))
  (bind _returnvalue (Transformation|GetActorLocation))
  (if (Variables|Default|GetDead)
    (if (Variables|Default|GetBy%20Eagle)
      (bind _output_get (Variables|Default|SetCamera%20Rotation%20Placeholder (Math|Interpolation|RInterpTo (Variables|Default|GetCamera%20Rotation%20Placeholder) "-80.000000, 0, 0" DeltaSeconds 1.5)))
      (Transformation|SetWorldRotation (Variables|Default|GetCamera) _output_get false false)
      (if (< (Transformation|GetDistanceTo (stale _eagle)) 5e+01)
        (Components|DestroyComponent (Variables|Default|GetChicken))
        (Audio|PlaySound2D "/Game/Sounds/eaglehit.eaglehit" 1.0 1.0 0.0 0 0)
        (Variables|Default|SetBy%20Eagle false)))
    (else
      (bind _eagle (CallFunction|CameraMovement DeltaSeconds))
      (if (Variables|Default|GetOn%20Log)
        (Variables|Default|SetLocation%20Placeholder (Math|Vector|MakeVector (.x (Math|Interpolation|VInterptoConstant (Variables|Default|GetLocation%20Placeholder) (Variables|Default|GetNew%20Position) DeltaSeconds 5e+02)) (.y _returnvalue) (.z _returnvalue)))
        (else
          (bind _output_get_2 (Variables|Default|SetLocation%20Placeholder (Math|Vector|MakeVector (.x (Math|Interpolation|VInterptoConstant (Variables|Default|GetLocation%20Placeholder) (Variables|Default|GetNew%20Position) DeltaSeconds 5e+02)) (.y (Math|Interpolation|VInterptoConstant (Variables|Default|GetLocation%20Placeholder) (Variables|Default|GetNew%20Position) DeltaSeconds 5e+02)) (.z _returnvalue))))))
      (bind _returnvalue_2 (Transformation|SetActorLocation _output_get_2 true false))
      (if _returnvalue_2
        _
        (else
          (Variables|Default|SetNew%20Position (Variables|Default|GetLast%20Position))))
      (bind _output_get_3 (Variables|Default|SetRotation%20Placeholder (Class|KismetMathLibrary|RInterptoConstant (Variables|Default|GetRotation%20Placeholder) (Variables|Default|GetNew%20Rotation) DeltaSeconds 5e+02)))
      (Transformation|SetActorRotation _output_get_3)
      (if (>= (.x (Transformation|GetActorLocation)) (Variables|Default|GetFurthest%20Distance))
        (Variables|Default|SetFurthest%20Distance (.x (Transformation|GetActorLocation))))
      (Variables|/Game/Blueprints/UIStuff/Score.Score_C|SetDisplayScore (stale EventBeginPlay _returnvalue) (/ (Math|Float|Round (Variables|Default|GetFurthest%20Distance)) (Math|Float|Truncate (Variables|Default|GetMovementSteps))))
      (if (> (Math|Float|Absolute(Float) (.y (Transformation|GetActorLocation))) 496.0)
        (if (Variables|Default|GetOn%20Log)
          (Components|DestroyComponent (Variables|Default|GetChicken))
          (Variables|Default|SetDead true)
          (else
            (Variables|Default|SetNew%20Position (Variables|Default|GetLast%20Position))))))))

(event Collision|EventHit
  (params (MyComp :type Primitive%20Component%20Object%20Reference) (Other :type Actor%20Object%20Reference) (OtherComp :type Primitive%20Component%20Object%20Reference) (bSelfMoved :type Boolean) (HitLocation :type Vector :default "0, 0, 0") (HitNormal :type Vector :default "0, 0, 0") (NormalImpulse :type Vector :default "0, 0, 0") (Hit :type Hit%20Result%20Structure%20%28by%20ref%29))
  (bind _particlesystem (Variables|Default|GetParticleSystem))
  (Utilities|Casting|CastToCar_Move Other
    (:then
      (if (not (Variables|Default|GetDead)) :!label _label
        (CallFunction|ChickenSquish Hit Other)
        (Audio|PlaySound2D "/Game/Sounds/carhit.carhit" 1.0 1.0 0.0 0 0)
        (Effects|Components|ParticleSystem|SetTemplate _particlesystem "/Game/Blueprints/SplashEffect/DeathExplosion.DeathExplosion" :!label _label_2)
        (Components|Activation|Activate _particlesystem false)
        (if (< (Math|Random|RandomIntegerinRange 0 100) 50) :!label _label_3
          (Audio|PlaySound2D "/Game/Sounds/chickendeath.chickendeath" 1.0 1.0 0.0 0 0)
          (else
            (Audio|PlaySound2D "/Game/Sounds/chickendeath2.chickendeath2" 1.0 1.0 0.0 0 0)))
        (Variables|Default|SetDead true)))
    (:CastFailed
      (Utilities|Casting|CastToTruck_Move Other
        (:then
          (goto _label))
        (:CastFailed
          (Utilities|Casting|CastToTrain_Move Other
            (:then
              (if (not (Variables|Default|GetDead))
                (Audio|PlaySound2D "/Game/Sounds/trainsplat.trainsplat" 1.0 1.0 0.0 0 0)
                (Components|DestroyComponent (Variables|Default|GetChicken))
                (goto _label_2)))
            (:CastFailed
              (Utilities|Casting|CastToWater Other
                (:then
                  (if (not (Variables|Default|GetDead))
                    (Audio|PlaySound2D "/Game/Sounds/watersplashlow.watersplashlow" 1.0 1.0 0.0 0 0)
                    (Components|Activation|Activate (Variables|Default|GetParticleSystem) false)
                    (Components|DestroyComponent (Variables|Default|GetChicken))
                    (goto _label_3)))
                (:CastFailed
                  (bind _aslog_move (Utilities|Casting|CastToLog_Move Other)
                    (:then
                      (if (< (Math|Random|RandomIntegerinRange 0 100) 50)
                        (Audio|Components|Audio|SetSound (Variables|/Game/Blueprints/Log_Move.Log_Move_C|GetAudio _aslog_move) "/Game/Sounds/logjump3.logjump3")
                        (else
                          (Audio|Components|Audio|SetSound (Variables|/Game/Blueprints/Log_Move.Log_Move_C|GetAudio _aslog_move) "/Game/Sounds/logjump4.logjump4")))
                      (Audio|Components|Audio|Play (Variables|/Game/Blueprints/Log_Move.Log_Move_C|GetAudio _aslog_move) 0.0)
                      (Variables|Default|SetOn%20Log true))
                    (:CastFailed
                      (bind _aslilypad (Utilities|Casting|CastToLilypad Other))
                      (Audio|Components|Audio|Play (Variables|/Game/Blueprints/Lilypad.Lilypad_C|GetAudio _aslilypad) 0.0))))))))))))

(event Input|ActionEvents|InputActionMoveUp
  (params (Key :type Key%20Structure))
  (:Pressed
    (if (not (Variables|Default|GetDead))
      (Transformation|SetWorldScale3D (Variables|Default|GetChicken) "12.000000,12.000000,5.000000")))
  (:Released
    (if (not (Variables|Default|GetDead))
      (Variables|Default|SetLast%20Position (Variables|Default|GetNew%20Position))
      (Variables|Default|SetNew%20Position (+ (Variables|Default|GetNew%20Position) (Math|Vector|MakeVector (Variables|Default|GetMovementSteps) 0.0 0.0)))
      (Variables|Default|SetNew%20Rotation "0, 0, 0")
      (Character|Jump)
      (if (Variables|Default|GetOn%20Log)
        (Variables|Default|SetOn%20Log false)
        (Variables|Default|SetNew%20Position (Math|Vector|MakeVector (.x (Variables|Default|GetNew%20Position)) (* (Math|Float|Round (/ (.y (Transformation|GetActorLocation)) 1e+02)) 1e+02) (.z (Variables|Default|GetNew%20Position)))))
      (Transformation|SetWorldScale3D (Variables|Default|GetChicken) "10.000000,10.000000,10.000000")
      (switch int (Math|Random|RandomIntegerinRange 0 12)
        (:Default
          (Audio|PlaySound2D "/Game/Sounds/buck1.buck1" 1.0 1.0 0.0 0 0 :!label _label))
        (:0
          (goto _label))
        (:1
          (Audio|PlaySound2D "/Game/Sounds/buck2.buck2" 1.0 1.0 0.0 0 0))
        (:2
          (Audio|PlaySound2D "/Game/Sounds/buck3.buck3" 1.0 1.0 0.0 0 0))
        (:3
          (Audio|PlaySound2D "/Game/Sounds/buck4.buck4" 1.0 1.0 0.0 0 0))
        (:4
          (Audio|PlaySound2D "/Game/Sounds/buck5.buck5" 1.0 1.0 0.0 0 0))
        (:5
          (Audio|PlaySound2D "/Game/Sounds/buck6.buck6" 1.0 1.0 0.0 0 0))
        (:6
          (Audio|PlaySound2D "/Game/Sounds/buck7.buck7" 1.0 1.0 0.0 0 0))
        (:7
          (Audio|PlaySound2D "/Game/Sounds/buck8.buck8" 1.0 1.0 0.0 0 0))
        (:8
          (Audio|PlaySound2D "/Game/Sounds/buck9.buck9" 1.0 1.0 0.0 0 0))
        (:9
          (Audio|PlaySound2D "/Game/Sounds/buck10.buck10" 1.0 1.0 0.0 0 0))
        (:10
          (Audio|PlaySound2D "/Game/Sounds/buck11.buck11" 1.0 1.0 0.0 0 0))
        (:11
          (Audio|PlaySound2D "/Game/Sounds/buck12.buck12" 1.0 1.0 0.0 0 0))))))

(event Input|ActionEvents|InputActionMoveDown
  (params (Key :type Key%20Structure))
  (:Pressed
    (if (not (Variables|Default|GetDead))
      (Transformation|SetWorldScale3D (Variables|Default|GetChicken) "12.000000,12.000000,5.000000")))
  (:Released
    (if (not (Variables|Default|GetDead))
      (Variables|Default|SetLast%20Position (Variables|Default|GetNew%20Position))
      (Variables|Default|SetNew%20Position (+ (Variables|Default|GetNew%20Position) (Math|Vector|MakeVector (* (Variables|Default|GetMovementSteps) -1.0) 0.0 0.0)))
      (Variables|Default|SetNew%20Rotation "0,180.000000, 0")
      (Character|Jump)
      (if (Variables|Default|GetOn%20Log)
        (Variables|Default|SetOn%20Log false)
        (Variables|Default|SetNew%20Position (Math|Vector|MakeVector (.x (Variables|Default|GetNew%20Position)) (* (Math|Float|Round (/ (.y (Transformation|GetActorLocation)) 1e+02)) 1e+02) (.z (Variables|Default|GetNew%20Position)))))
      (Transformation|SetWorldScale3D (Variables|Default|GetChicken) "10.000000,10.000000,10.000000")
      (switch int (Math|Random|RandomIntegerinRange 0 12)
        (:Default
          (Audio|PlaySound2D "/Game/Sounds/buck1.buck1" 1.0 1.0 0.0 0 0 :!label _label))
        (:0
          (goto _label))
        (:1
          (Audio|PlaySound2D "/Game/Sounds/buck2.buck2" 1.0 1.0 0.0 0 0))
        (:2
          (Audio|PlaySound2D "/Game/Sounds/buck3.buck3" 1.0 1.0 0.0 0 0))
        (:3
          (Audio|PlaySound2D "/Game/Sounds/buck4.buck4" 1.0 1.0 0.0 0 0))
        (:4
          (Audio|PlaySound2D "/Game/Sounds/buck5.buck5" 1.0 1.0 0.0 0 0))
        (:5
          (Audio|PlaySound2D "/Game/Sounds/buck6.buck6" 1.0 1.0 0.0 0 0))
        (:6
          (Audio|PlaySound2D "/Game/Sounds/buck7.buck7" 1.0 1.0 0.0 0 0))
        (:7
          (Audio|PlaySound2D "/Game/Sounds/buck8.buck8" 1.0 1.0 0.0 0 0))
        (:8
          (Audio|PlaySound2D "/Game/Sounds/buck9.buck9" 1.0 1.0 0.0 0 0))
        (:9
          (Audio|PlaySound2D "/Game/Sounds/buck10.buck10" 1.0 1.0 0.0 0 0))
        (:10
          (Audio|PlaySound2D "/Game/Sounds/buck11.buck11" 1.0 1.0 0.0 0 0))
        (:11
          (Audio|PlaySound2D "/Game/Sounds/buck12.buck12" 1.0 1.0 0.0 0 0))))))

(event Input|ActionEvents|InputActionMoveLeft
  (params (Key :type Key%20Structure))
  (:Pressed
    (if (not (Variables|Default|GetDead))
      (Transformation|SetWorldScale3D (Variables|Default|GetChicken) "12.000000,12.000000,5.000000")))
  (:Released
    (if (not (Variables|Default|GetDead))
      (Variables|Default|SetLast%20Position (Variables|Default|GetNew%20Position))
      (Variables|Default|SetNew%20Position (+ (Variables|Default|GetNew%20Position) (Math|Vector|MakeVector 0.0 (* (Variables|Default|GetMovementSteps) -1.0) 0.0)))
      (Variables|Default|SetNew%20Rotation "0,270.000000, 0")
      (Character|Jump)
      (if (Variables|Default|GetOn%20Log)
        (Variables|Default|SetOn%20Log false)
        (Variables|Default|SetNew%20Position (Math|Vector|MakeVector (.x (Variables|Default|GetNew%20Position)) (* (Math|Float|Round (/ (.y (Transformation|GetActorLocation)) 1e+02)) 1e+02) (.z (Variables|Default|GetNew%20Position)))))
      (Transformation|SetWorldScale3D (Variables|Default|GetChicken) "10.000000,10.000000,10.000000")
      (switch int (Math|Random|RandomIntegerinRange 0 12)
        (:Default
          (Audio|PlaySound2D "/Game/Sounds/buck1.buck1" 1.0 1.0 0.0 0 0 :!label _label))
        (:0
          (goto _label))
        (:1
          (Audio|PlaySound2D "/Game/Sounds/buck2.buck2" 1.0 1.0 0.0 0 0))
        (:2
          (Audio|PlaySound2D "/Game/Sounds/buck3.buck3" 1.0 1.0 0.0 0 0))
        (:3
          (Audio|PlaySound2D "/Game/Sounds/buck4.buck4" 1.0 1.0 0.0 0 0))
        (:4
          (Audio|PlaySound2D "/Game/Sounds/buck5.buck5" 1.0 1.0 0.0 0 0))
        (:5
          (Audio|PlaySound2D "/Game/Sounds/buck6.buck6" 1.0 1.0 0.0 0 0))
        (:6
          (Audio|PlaySound2D "/Game/Sounds/buck7.buck7" 1.0 1.0 0.0 0 0))
        (:7
          (Audio|PlaySound2D "/Game/Sounds/buck8.buck8" 1.0 1.0 0.0 0 0))
        (:8
          (Audio|PlaySound2D "/Game/Sounds/buck9.buck9" 1.0 1.0 0.0 0 0))
        (:9
          (Audio|PlaySound2D "/Game/Sounds/buck10.buck10" 1.0 1.0 0.0 0 0))
        (:10
          (Audio|PlaySound2D "/Game/Sounds/buck11.buck11" 1.0 1.0 0.0 0 0))
        (:11
          (Audio|PlaySound2D "/Game/Sounds/buck12.buck12" 1.0 1.0 0.0 0 0))))))

(event Input|ActionEvents|InputActionMoveRight
  (params (Key :type Key%20Structure))
  (:Pressed
    (if (not (Variables|Default|GetDead))
      (Transformation|SetWorldScale3D (Variables|Default|GetChicken) "12.000000,12.000000,5.000000")))
  (:Released
    (if (not (Variables|Default|GetDead))
      (Variables|Default|SetLast%20Position (Variables|Default|GetNew%20Position))
      (Variables|Default|SetNew%20Position (+ (Variables|Default|GetNew%20Position) (Math|Vector|MakeVector 0.0 (Variables|Default|GetMovementSteps) 0.0)))
      (Variables|Default|SetNew%20Rotation "0,90.000000, 0")
      (Character|Jump)
      (if (Variables|Default|GetOn%20Log)
        (Variables|Default|SetOn%20Log false)
        (Variables|Default|SetNew%20Position (Math|Vector|MakeVector (.x (Variables|Default|GetNew%20Position)) (* (Math|Float|Round (/ (.y (Transformation|GetActorLocation)) 1e+02)) 1e+02) (.z (Variables|Default|GetNew%20Position)))))
      (Transformation|SetWorldScale3D (Variables|Default|GetChicken) "10.000000,10.000000,10.000000")
      (switch int (Math|Random|RandomIntegerinRange 0 12)
        (:Default
          (Audio|PlaySound2D "/Game/Sounds/buck1.buck1" 1.0 1.0 0.0 0 0 :!label _label))
        (:0
          (goto _label))
        (:1
          (Audio|PlaySound2D "/Game/Sounds/buck2.buck2" 1.0 1.0 0.0 0 0))
        (:2
          (Audio|PlaySound2D "/Game/Sounds/buck3.buck3" 1.0 1.0 0.0 0 0))
        (:3
          (Audio|PlaySound2D "/Game/Sounds/buck4.buck4" 1.0 1.0 0.0 0 0))
        (:4
          (Audio|PlaySound2D "/Game/Sounds/buck5.buck5" 1.0 1.0 0.0 0 0))
        (:5
          (Audio|PlaySound2D "/Game/Sounds/buck6.buck6" 1.0 1.0 0.0 0 0))
        (:6
          (Audio|PlaySound2D "/Game/Sounds/buck7.buck7" 1.0 1.0 0.0 0 0))
        (:7
          (Audio|PlaySound2D "/Game/Sounds/buck8.buck8" 1.0 1.0 0.0 0 0))
        (:8
          (Audio|PlaySound2D "/Game/Sounds/buck9.buck9" 1.0 1.0 0.0 0 0))
        (:9
          (Audio|PlaySound2D "/Game/Sounds/buck10.buck10" 1.0 1.0 0.0 0 0))
        (:10
          (Audio|PlaySound2D "/Game/Sounds/buck11.buck11" 1.0 1.0 0.0 0 0))
        (:11
          (Audio|PlaySound2D "/Game/Sounds/buck12.buck12" 1.0 1.0 0.0 0 0))))))

(event Input|KeyboardEvents|R
  (params (Key :type Key%20Structure))
  (:Pressed
    (if (Variables|Default|GetDead)
      (Variables|Default|SetI%20Want%20to%20Restart true))))

(fn ConstructionScript)

(fn CameraMovement
  (params (Delta%20Seconds :type Float%20%28single-precision%29))
  (bind _returnvalue (Transformation|GetActorLocation))
  (bind _returnvalue_2 (Transformation|GetActorLocation))
  (bind _camera (Variables|Default|GetCamera))
  (bind _camera_2 (Variables|Default|GetCamera))
  (bind _returnvalue_3 (Transformation|GetWorldLocation _camera))
  (bind _returnvalue_4 (Transformation|GetWorldLocation _camera_2))
  (bind _returnvalue_5 (- (.x _returnvalue_4) (.x _returnvalue)))
  (bind _returnvalue_6 (Math|Float|Absolute(Float) _returnvalue_5))
  (Transformation|AddLocalOffset _camera (Math|Vector|MakeVector (* _returnvalue_6 Delta%20Seconds 0.25) 0.0 0.0) false false)
  (Transformation|SetWorldLocation _camera (Math|Vector|MakeVector (.x _returnvalue_3) (.y _returnvalue_3) 5.5e+02) false false)
  (if (< _returnvalue_6 2e+02)
    (bind _returnvalue_7 (Game|SpawnActorfromClass "/Game/Blueprints/Eagle.Eagle_C" (Math|Conversions|ToTransform(Vector) (Math|Vector|MakeVector (+ (.x _returnvalue_2) 1e+03) (.y _returnvalue_2) 5e+02)) "Undefined" 0 0))
    (Audio|PlaySound2D "/Game/Sounds/hawk-screech-02.hawk-screech-02" 1.0 1.0 0.0 0 0)
    (Variables|Default|SetDead true)
    (Variables|Default|SetBy%20Eagle true)
    (return _returnvalue_7)))

(fn ChickenSquish
  (params (Hit :type Hit%20Result%20Structure) (Actor%20Stuck :type Actor%20Object%20Reference))
  (bind _chicken (Variables|Default|GetChicken))
  (if (< (Math|Float|Absolute(Float) (Class|KismetMathLibrary|DegAsin (Math|Vector|DotProduct (.Normal (Collision|BreakHitResult Hit)) (Math|Vector|GetRightVector (Variables|Collision|GetCapsuleComponent))))) 45.0)
    (Transformation|SetWorldScale3D _chicken "1.000000,15.000000,15.000000")
    (Transformation|AttachActorToActor Actor%20Stuck "None" "KeepWorld" "KeepWorld" "KeepWorld" true)
    (else
      (Transformation|SetWorldScale3D _chicken "15.000000,15.000000,1.000000")
      (Collision|SetActorEnableCollision false))))